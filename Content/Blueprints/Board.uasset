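; Board actor that builds a checkered, square grid of BoardSquareA actors at BeginPlay, apparently for a piece-based game.
; The first square spawns at the board's transform; its bounds set the spacing for the rest, all attached to the board.
; Index parity picks black or white material, and a flattened array stores squares for lookup by X/Y and center position.
; Occupancy and piece queries are empty stubs.
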(event EventBeginPlay
  (bind _squarecount (Variables|Default|GetSquareCount))
  (bind _output_get (Variables|Default|SetSquares (Utilities|Array|MakeArray 0)))
  (Utilities|Array|Resize _output_get (* _squarecount 2))
  (CallFunction|CreateBoard _squarecount))

(fn ConstructionScript)

(fn CreateBoard
  (params (squareCount :type Integer))
  (bind _returnvalue (- squareCount 1))
  (for _index (range 0 _returnvalue)
    (for _index_2 (range 0 _returnvalue)
      (if (and (== _index 0) (== _index_2 0))
        ;[1 1 1] Create first square only
        (bind _returnvalue_2 (Game|SpawnActorfromClass "/Game/Blueprints/BoardSquareA.BoardSquareA_C" (Transformation|GetActorTransform) "Undefined" 0 0))
        (bind _output_get (LocalVariables|SetLastSpawnedSquare _returnvalue_2))
        (Class|Actor|AttachRootComponenttoActor _output_get self "None" "KeepWorldPosition" true)
        (LocalVariables|SetSquareExtents (.BoxExtent (Collision|GetActorBounds _returnvalue_2 false)))
        (LocalVariables|SetFirstLocation (Transformation|GetActorLocation _returnvalue_2))
        (CallFunction|SetAlternatingMaterial (Utilities|Array|Get(acopy) (Actor|GetComponentsByClass (LocalVariables|GetLastSpawnedSquare) "/Script/Engine.StaticMeshComponent")) _index _index_2 :!label _label)
        (bind _asboard_square_a (Utilities|Casting|CastToBoardSquareA (LocalVariables|GetLastSpawnedSquare)))
        (CallFunction|SetSquareatIndex _index _index_2 _asboard_square_a)
        (else
          ;[1 1 1] Create all squares, except the first
          (bind _returnvalue_3 (Game|SpawnActorfromClass "/Game/Blueprints/BoardSquareA.BoardSquareA_C" (Math|Transform|MakeTransform (Math|Vector|MakeVector (+ (* _index (* (.X (Math|Vector|BreakVector (LocalVariables|GetSquareExtents))) 2.0)) (.X (Math|Vector|BreakVector (LocalVariables|GetFirstLocation)))) (+ (* _index_2 (* (.Y (Math|Vector|BreakVector (LocalVariables|GetSquareExtents))) 2.0)) (.Y (Math|Vector|BreakVector (LocalVariables|GetFirstLocation)))) (.Z (Math|Vector|BreakVector (LocalVariables|GetFirstLocation))))) "Undefined" 0 0))
          (bind _output_get_2 (LocalVariables|SetLastSpawnedSquare _returnvalue_3))
          (Class|Actor|AttachRootComponenttoActor _output_get_2 self "None" "KeepWorldPosition" true)
          (if true
            (Development|PrintString "Spawned")
            (Development|PrintString (Utilities|String|ToString(Vector) (Math|Vector|MakeVector (+ (* _index (* (.X (Math|Vector|BreakVector (LocalVariables|GetSquareExtents))) 2.0)) (.X (Math|Vector|BreakVector (LocalVariables|GetFirstLocation)))) (+ (* _index_2 (* (.Y (Math|Vector|BreakVector (LocalVariables|GetSquareExtents))) 2.0)) (.Y (Math|Vector|BreakVector (LocalVariables|GetFirstLocation)))) (.Z (Math|Vector|BreakVector (LocalVariables|GetFirstLocation))))))
            (goto _label)
            (else
              (Development|PrintString "Not Spawned"))))))))

(fn SetAlternatingMaterial
  (params (Mesh :type Static%20Mesh%20Component%20Object%20Reference) (X :type Integer) (Y :type Integer))
  (if (or (and (== (Math|Integer|%(Integer) X 2) 0) (== (Math|Integer|%(Integer) Y 2) 0)) (and (== (Math|Integer|%(Integer) X 2) 1) (== (Math|Integer|%(Integer) Y 2) 1)))
    (Rendering|Material|SetMaterial Mesh 0 (Variables|Default|GetBlackMaterial))
    (else
      (Rendering|Material|SetMaterial Mesh 0 (Variables|Default|GetWhiteMaterial)))))

(fn SetSquareatIndex
  (params (X :type Integer) (Y :type Integer) (Square :type Board%20Square%20A%20Object%20Reference))
  (Utilities|Array|SetArrayElem (Variables|Default|GetSquares) (+ X (* Y (Variables|Default|GetSquareCount))) Square true))

(fn GetSquareatIndex
  (params (X :type Integer) (Y :type Integer))
  (return (Utilities|Array|Get(acopy) (Variables|Default|GetSquares) (+ X (* Y (Variables|Default|GetSquareCount))))))

(fn GetCenterOfIndex
  (params (X :type Integer) (Y :type Integer))
  (bind _square (CallFunction|GetSquareatIndex X Y))
  (return (Math|Vector|MakeVector (.X (Math|Vector|BreakVector (.Origin (Collision|GetActorBounds _square false)))) (.Y (Math|Vector|BreakVector (.Origin (Collision|GetActorBounds _square false)))) (.Z (Math|Vector|BreakVector (.BoxExtent (Collision|GetActorBounds _square false)))))))

(fn IndexIsOccupied
  (params (Index :type Array%20of%20Integers))
  (return false))

(fn PieceatIndex
  (params (Index :type Array%20of%20Integers))
  (return 0))