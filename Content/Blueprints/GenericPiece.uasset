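; GenericPiece is a grabbable piece actor that, when not held, returns to its starting rotation and glides toward a TargetLocation.
; Mesh overlaps cache any Grabber-interface actor, which receives a PickupMessage every tick, while OnGrab and OnRelease toggle the Grabbed state.
; Tick interpolates rotation and XY position, leaving Z to physics, but teleports the piece just above the target if it drops below it.
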(event `self.ReceiveBeginPlay`
  (set `self.StartingRotation` (`self.K2_GetActorRotation`)))

(event `self.ReceiveTick`
  (params (DeltaSeconds :type "Float (single-precision)"))
  (message `/Game/Blueprints/Grabber.Pickup` (`self.OverlappingGrabber`) self (`self.OverlapLocation`))
  (if (not (`self.Grabbed`))
    (if (not (== (`self.StartingRotation`) (`self.K2_GetActorRotation`)))
      (`self.RotateToStartRotation`))
    (if (not (== (`self.TargetLocation`) (`self.K2_GetActorLocation`)))
      (`self.InterpolateXYToPosition`)
      (if (> (- (.z (`self.TargetLocation`)) (.z (`self.K2_GetActorLocation`))) 0.0)
        (`self.TeleportAboveTarget`)))))

(event `self.StaticMeshComponent.OnComponentBeginOverlap`
  (params (OtherActor :type "Actor Object Reference") (OtherComp :type "PrimitiveComponent Object Reference") (OtherBodyIndex :type Integer) (bFromSweep :type Boolean) (SweepResult :type "HitResult Structure (by ref)"))
  (if (`KismetSystemLibrary.DoesImplementInterface` OtherActor "/Game/Blueprints/Grabber.Grabber_C")
    (set `self.OverlappingGrabber` OtherActor)
    (set `self.OverlapLocation` (`.Location` (`GameplayStatics.BreakHitResult` SweepResult)))))

(event `self.StaticMeshComponent.OnComponentEndOverlap`
  (params (OtherActor :type "Actor Object Reference") (OtherComp :type "PrimitiveComponent Object Reference") (OtherBodyIndex :type Integer))
  (set `self.OverlappingGrabber` null)
  (set `self.OverlapLocation` (0.0 0.0 0.0)))

(event `/Game/Blueprints/Grabbable.OnRelease`
  (set `self.Grabbed` false))

(event `/Game/Blueprints/Grabbable.OnGrab`
  (params (Grabber :type "/Game/Blueprints/Grabber Interface"))
  (set `self.Grabbed` true))

(fn `InterpolateXYToPosition`
  (bind _returnvalue (`self.K2_GetActorLocation`))
  (`self.K2_SetActorLocation` (`KismetMathLibrary.MakeVector` (.x (`KismetMathLibrary.VInterpTo` _returnvalue (`self.TargetLocation`) (`GameplayStatics.GetWorldDeltaSeconds`) 10.0)) (.y (`KismetMathLibrary.VInterpTo` _returnvalue (`self.TargetLocation`) (`GameplayStatics.GetWorldDeltaSeconds`) 10.0)) (.z _returnvalue)) false true))

(fn `RotateToStartRotation`
  (`self.SetActorRotation` (`KismetMathLibrary.RInterpTo` (`self.K2_GetActorRotation`) (`self.StartingRotation`) (`GameplayStatics.GetWorldDeltaSeconds`) 20.0)))

(fn `TeleportAboveTarget`
  (`self.K2_SetActorLocation` (`KismetMathLibrary.MakeVector` (.x (`self.K2_GetActorLocation`)) (.y (`self.K2_GetActorLocation`)) (+ (.z (`self.TargetLocation`)) (.z (`.BoxExtent` (`self.GetActorBounds` false))) 10.0)) false true)
  (return))

(fn `UserConstructionScript`)