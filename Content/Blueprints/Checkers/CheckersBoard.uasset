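; Checkers board actor that spawns and tracks red and black pieces and runs captures, king promotion and game over.
; Move legality and turns are delegated to CheckersRules, with JumpingPiece restricting play to the piece mid multi-jump.
; The server spawns the starting layout after a delay and saves a checkpoint, which F restores once by respawning pieces.
; Tick polls GameOver to destroy all pieces and start a new game.
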(event EventBeginPlay
  (|CallParentFunction)
  (Utilities|FlowControl|Delay 1.0) ; Delay to allow board to finish spawning. TODO: spawn pieces after a callback indicates the board is spawned
  (if (Networking|IsServer)
    (CallFunction|SpawnPieces)
    (CallFunction|SaveState))
  (Input|EnableInput (Game|GetPlayerController 0)))

(event EventActorBeginOverlap
  (params (OtherActor :type Actor%20Object%20Reference)))

(event EventTick
  (params (DeltaSeconds :type Float%20%28single-precision%29))
  (bind _blackpieces (Variables|CheckersProperties|GetBlackPieces))
  (bind _redpieces (Variables|CheckersProperties|GetRedPieces))
  (if (Variables|CheckersProperties|GetGameOver)
    (Variables|CheckersProperties|SetGameOver false)
    (Utilities|FlowControl|Delay 1.0)
    (for _array_element (Variables|CheckersProperties|GetBlackPieces)
      (bind _asactor (Utilities|Casting|CastToActor _array_element))
      (Actor|DestroyActor _asactor))
    (for _array_element_2 (Variables|CheckersProperties|GetRedPieces)
      (bind _asactor_2 (Utilities|Casting|CastToActor _array_element_2))
      (Actor|DestroyActor _asactor_2))
    (Utilities|Array|Clear _blackpieces)
    (Utilities|Array|Resize _blackpieces 0)
    (Utilities|Array|Clear _redpieces)
    (Utilities|Array|Resize _redpieces 0)
    (Variables|CheckersProperties|SetJumpingPiece 0)
    (Variables|CheckersProperties|SetGameOver false)
    (Variables|/Game/Blueprints/Checkers/CheckersRules.CheckersRules_C|SetBlacksMove (Variables|Default|GetCheckersRules) true)
    (Variables|BoardSaves|SetSavedState "")
    (Variables|BoardSaves|SetSavedStateValid false)
    (CallFunction|SpawnPieces)))

(event Input|KeyboardEvents|F
  (params (Key :type Key%20Structure :default "AnyKey"))
  (:Pressed
    (bind _wasloaded (CallFunction|ReverttoCheckpoint))
    (if _wasloaded
      (Development|PrintString "Checkpoint loaded.")
      (else
        (Development|PrintString "No Checkpoint to load.")))))

(fn ConstructionScript)

(fn SpawnPieces
  (for _index (range 0 7)
    (for _index_2 (range 0 7)
      (bind _black (CallFunction|IndexIsBlack _index_2 _index))
      (if _black
        (if (< _index 3)
          (CallFunction|SpawnSinglePiece _index_2 _index true false)
          (elif (> _index 4)
            (CallFunction|SpawnSinglePiece _index_2 _index false false)))))))

(fn PieceatIndex
  (params (X :type Integer) (Y :type Integer))
  (for _array_element (Variables|CheckersProperties|GetBlackPieces)
    (bind (_x _y) (Default|GetIndex _array_element))
    (if (and (== _x X) (== _y Y))
      (return _array_element)))
  (for _array_element_2 (Variables|CheckersProperties|GetRedPieces)
    (bind (_x_2 _y_2) (Default|GetIndex _array_element_2))
    (if (and (== _x_2 X) (== _y_2 Y))
      (return _array_element_2)))
  (return 0))

(fn CapturePiece
  (params (Piece :type I%20Checkers%20Piece%20Interface))
  (if (!= (Utilities|ToObject(Interface) Piece) 0)
    (bind _returnvalue (Utilities|Array|RemoveItem (Variables|CheckersProperties|GetBlackPieces) Piece))
    (if _returnvalue
      (Default|Despawn Piece :!label _label)
      (else
        (bind _returnvalue_2 (Utilities|Array|RemoveItem (Variables|CheckersProperties|GetRedPieces) Piece))
        (if _returnvalue_2
          (goto _label))))))

(fn IndexIsOccupied
  (params (X :type Integer) (Y :type Integer))
  (bind _piece (CallFunction|PieceatIndex X Y))
  (return (!= (Utilities|ToObject(Interface) _piece) 0)))

(fn CanMakeMove
  (params (Piece :type I%20Checkers%20Piece%20Interface) (TargetX :type Integer) (TargetY :type Integer))
  (bind _jumpingpiece (Variables|CheckersProperties|GetJumpingPiece))
  (bind _returnvalue (Utilities|ToObject(Interface) _jumpingpiece))
  (if (or (== _returnvalue 0) (== (Utilities|ToObject(Interface) Piece) _returnvalue))
    (bind (_legalmove _piecetocapture) (Default|CanMovePiece (Variables|Default|GetCheckersRules) Piece self TargetX TargetY))
    (return _legalmove _piecetocapture)
    (else
      (return false 0))))

(fn SaveState
  (for _array_element (Variables|CheckersProperties|GetRedPieces)
    (bind (_x _y) (Default|GetIndex _array_element))
    (bind _king (Default|IsKing _array_element))
    (Utilities|Array|Add (LocalVariables|GetTempEntryArray) (Utilities|Struct|MakeCheckersSaveEntry _x _y _king false)))
  (for _array_element_2 (Variables|CheckersProperties|GetBlackPieces)
    (bind (_x_2 _y_2) (Default|GetIndex _array_element_2))
    (bind _king_2 (Default|IsKing _array_element_2))
    (Utilities|Array|Add (LocalVariables|GetTempEntryArray) (Utilities|Struct|MakeCheckersSaveEntry _x_2 _y_2 _king_2 true)))
  (Variables|BoardSaves|SetSavedState (Utilities|Struct|MakeCheckersSaveState (LocalVariables|GetTempEntryArray)))
  (Variables|BoardSaves|SetSavedStateValid true)
  (Development|PrintString "Checkpoint Saved.")
  (return))

(fn SwitchPlayers
  (Default|SwitchPlayers (Variables|Default|GetCheckersRules)))

(fn MakeMove
  (params (PieceToMove :type I%20Checkers%20Piece%20Interface) (X :type Integer) (Y :type Integer) (CapturedPiece :type I%20Checkers%20Piece%20Interface))
  (bind _black (Default|IsBlack PieceToMove))
  (if (or (and _black (== Y 7)) (and (not _black) (== Y 0)))
    (Default|MakeKing PieceToMove))
  (if (== (Utilities|ToObject(Interface) CapturedPiece) 0)
    (return false)
    (else
      (CallFunction|CapturePiece CapturedPiece)
      (bind _gameover (CallFunction|CheckforGameOver))
      (if _gameover
        (CallFunction|EndGame)
        (return false)
        (else
          (bind _yindices (Default|GetLegalJumps (Variables|Default|GetCheckersRules) PieceToMove self))
          (if (> (Utilities|Array|Length _yindices) 0)
            (Variables|CheckersProperties|SetJumpingPiece PieceToMove)
            (else
              (Variables|CheckersProperties|SetJumpingPiece 0)))
          (return (> (Utilities|Array|Length _yindices) 0)))))))

(fn CheckforGameOver
  (return (or (== (Utilities|Array|Length (Variables|CheckersProperties|GetBlackPieces)) 0) (== (Utilities|Array|Length (Variables|CheckersProperties|GetRedPieces)) 0))))

(fn EndGame
  (Variables|CheckersProperties|SetGameOver true)
  (if (== (Utilities|Array|Length (Variables|CheckersProperties|GetBlackPieces)) 0)
    (Development|PrintString "Black Wins!")
    (elif (== (Utilities|Array|Length (Variables|CheckersProperties|GetRedPieces)) 0)
      (Development|PrintString "Red Wins!"))))

(fn DeletePieces
  (for _array_element (Variables|CheckersProperties|GetRedPieces)
    (Default|Despawn _array_element))
  (for _array_element_2 (Variables|CheckersProperties|GetBlackPieces)
    (Default|Despawn _array_element_2)))

(fn LoadState
  (params (savedState :type Checkers%20Save%20State%20Structure))
  (for _array_element (Utilities|Struct|BreakCheckersSaveState savedState)
    (CallFunction|SpawnSinglePiece (.X (Utilities|Struct|BreakCheckersSaveEntry _array_element)) (.Y (Utilities|Struct|BreakCheckersSaveEntry _array_element)) (.Black (Utilities|Struct|BreakCheckersSaveEntry _array_element)) (.King (Utilities|Struct|BreakCheckersSaveEntry _array_element))))
  (Variables|BoardSaves|SetSavedStateValid false)
  (return))

(fn ReverttoCheckpoint
  (if (Variables|BoardSaves|GetSavedStateValid)
    (CallFunction|DeletePieces)
    (CallFunction|LoadState (Variables|BoardSaves|GetSavedState))
    (return true)
    (else
      (return false))))

(fn SpawnSinglePiece
  (params (X :type Integer) (Y :type Integer) (Black :type Boolean) (King :type Boolean))
  (bind _self self)
  (bind _self_2 self)
  (bind _returnvalue (Transformation|GetActorTransform _self))
  (bind _returnvalue_2 (Transformation|GetActorTransform _self_2))
  (bind (_location _rotation _scale) (Math|Transform|BreakTransform _returnvalue))
  (bind (_location_2 _rotation_2 _scale_2) (Math|Transform|BreakTransform _returnvalue_2))
  (if Black
    ;[1 1 1] Spawn Black
    (bind _center (CallFunction|GetCenterOfIndex X Y))
    (bind _returnvalue_3 (Game|SpawnActorfromClass (Variables|CheckersProperties|GetPieceClass) (Math|Transform|MakeTransform (Math|Vector|MakeVector (.X (Math|Vector|BreakVector _center)) (.Y (Math|Vector|BreakVector _center)) (+ (.Z (Math|Vector|BreakVector _center)) 1e+01)) _rotation_2 _scale_2) "Undefined" 0 true self "/Game/Blueprints/Checkers/BlackCheckerMaterial.BlackCheckerMaterial" "/Game/Blueprints/Checkers/RedCheckerMaterial.RedCheckerMaterial" X Y))
    (Variables|/Game/Blueprints/Checkers/CheckersPiece.CheckersPiece_C|SetKing _returnvalue_3 King)
    (Utilities|Array|Add (Variables|CheckersProperties|GetBlackPieces) _returnvalue_3)
    (return _returnvalue_3)
    (else
      ;[1 1 1] Spawn Red
      (bind _center_2 (CallFunction|GetCenterOfIndex X Y))
      (bind _returnvalue_4 (Game|SpawnActorfromClass (Variables|CheckersProperties|GetPieceClass) (Math|Transform|MakeTransform (Math|Vector|MakeVector (.X (Math|Vector|BreakVector _center_2)) (.Y (Math|Vector|BreakVector _center_2)) (+ (.Z (Math|Vector|BreakVector _center_2)) 1e+01)) (Math|Rotator|CombineRotators _rotation "0,180.000000, 0") _scale) "Undefined" 0 (Class|KismetSystemLibrary|MakeLiteralBool false) self "/Game/Blueprints/Checkers/BlackCheckerMaterial.BlackCheckerMaterial" "/Game/Blueprints/Checkers/RedCheckerMaterial.RedCheckerMaterial" X Y))
      (Variables|/Game/Blueprints/Checkers/CheckersPiece.CheckersPiece_C|SetKing _returnvalue_4 King)
      (Utilities|Array|Add (Variables|CheckersProperties|GetRedPieces) _returnvalue_4)
      (return _returnvalue_4))))