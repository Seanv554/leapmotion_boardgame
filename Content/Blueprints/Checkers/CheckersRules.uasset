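; Checkers rules Blueprint whose CanMovePiece decides whether a piece may move to a target board cell.
; It queries the piece's king and colour state to check vertical direction, then accepts a one-step diagonal into an empty cell or a two-step jump over an opposite-coloured piece.
; A valid jump also captures the jumped piece on the board, so the check has a side effect.
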(event EventBeginPlay)

(event EventTick
  (params (DeltaSeconds :type Float%20%28single-precision%29)))

(fn CanMovePiece
  (params (Piece :type I%20Checkers%20Piece%20Interface) (Board :type Checkers%20Board%20Object%20Reference) (X :type Integer) (Y :type Integer))
  (bind _returnvalue (Utilities|ToObject(Interface) Piece))
  (bind (_x _y) (Default|GetIndex Piece))
  ;[1 1 1] Set dif local variables
  (bind _output_get (LocalVariables|SetxDif (- X _x)))
  (LocalVariables|SetxDifAbs (Math|Integer|Absolute(Integer) _output_get))
  (bind _output_get_2 (LocalVariables|SetyDif (- Y _y)))
  (LocalVariables|SetyDifAbs (Math|Integer|Absolute(Integer) _output_get_2))
  ;[1 1 1] Make sure the diagonal is in the right vertical direction
  (bind _king (Class|ICheckersPiece|IsKing(Message) _returnvalue))
  (if _king
    _
    (else
      (bind _black (Class|ICheckersPiece|IsBlack(Message) _returnvalue))))
  (if (or (and _black (> (LocalVariables|GetyDif) 0)) (and (not _black) (< (LocalVariables|GetyDif) 0)))
    ;[1 1 1] If move is 1 step diagonal to an open space
    (if (and (== (LocalVariables|GetxDifAbs) 1) (== (LocalVariables|GetyDifAbs) 1))
      (bind _occupied (Default|IndexIsOccupied Board X Y))
      (if _occupied
        (return false)
        (else
          _))
      (else
        ;[1 1 1] If move is 2 step diagonal, target index is open, and enemy piece is in the way
        (bind _occupied_2 (Default|IndexIsOccupied Board X Y))
        (bind _piece (Default|PieceatIndex Board (+ _x (/ (LocalVariables|GetxDif) 2)) (+ _y (/ (LocalVariables|GetyDif) 2))))
        ;;[1 1 1] Checking for None
        (if (not (== (Utilities|ToObject(Interface) _piece) 0))
          ;;[1 1 1] Check for dif. Colors
          (bind _black_2 (Class|ICheckersPiece|IsBlack(Message) (Utilities|ToObject(Interface) _piece)))
          (bind _black_3 (Class|ICheckersPiece|IsBlack(Message) (Utilities|ToObject(Interface) Piece)))
          (if (Math|Boolean|ANDBoolean (== (LocalVariables|GetxDifAbs) 2) (== (LocalVariables|GetyDifAbs) 2) (not _occupied_2) (Math|Boolean|Equal(Boolean) _black_2 (not _black_3)))
            (Default|CapturePiece Board _piece)
            (else
              (return false)))
          (else
            (return false)))))
    ;[1 1 1] Can Move the piece
    (return true)
    (else
      (return false))))