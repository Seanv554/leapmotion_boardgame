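; A grabbable checkers piece actor that tracks its board index, color and king status, with the server setting its initial target at the square center.
; While grabbed, Tick asks the Board whether the square below is a legal move and highlights it accordingly.
; On release, ValidateMove either commits the move or retargets the original square.
; When no further jumps remain, the piece has the Board save state and switch players.
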(event EventBeginPlay
  (bind _cube (Variables|Default|GetCube))
  (|CallParentFunction)
  (if (Networking|IsServer)
    (bind _center (Default|GetCenterOfIndex (Variables|Default|GetBoard) (Variables|Default|GetX) (Variables|Default|GetY)))
    (Variables|Default|SetTargetLocation _center))
  (if (Variables|Default|GetBlack)
    (Rendering|Material|SetMaterial _cube 0 (Variables|Default|GetBlackMaterial))
    (else
      (Rendering|Material|SetMaterial _cube 0 (Variables|Default|GetRedMaterial)))))

(event EventTick
  (params (DeltaSeconds :type Float%20%28single-precision%29))
  (|CallParentFunction DeltaSeconds)
  (if (Variables|Default|GetGrabbed)
    (bind _square (Default|GetSquareBelowPoint (Variables|Default|GetBoard) (Transformation|GetActorLocation)))
    (if (!= _square 0)
      (bind _legal_move (Default|CanMakeMove (Variables|Default|GetBoard) self (Variables|/Game/Blueprints/BoardSquare.BoardSquare_C|GetX _square) (Variables|/Game/Blueprints/BoardSquare.BoardSquare_C|GetY _square)))
      (CallFunction|SetSquareOver _square _legal_move))
    (else
      (CallFunction|ClearSquareOver))))

(event EventMakeKing
  (bind _kingcrown (Variables|Default|GetKingCrown))
  (Variables|Default|SetKing true)
  (Rendering|SetVisibility _kingcrown true false)
  (Rendering|Material|SetMaterial _kingcrown 0 (Rendering|Material|GetMaterial (Variables|Default|GetCube) 0)))

(event EventOnRelease
  (bind _board (Variables|Default|GetBoard))
  (|CallParentFunction)
  (bind (_mademove _morejumps) (CallFunction|ValidateMove))
  (if (and _mademove (not _morejumps))
    (Default|SaveState _board)
    (Default|SwitchPlayers _board)))

(fn ConstructionScript
  (|CallParentFunction))

(fn ValidateMove
  (bind _square (Default|GetSquareBelowPoint (Variables|Default|GetBoard) (Transformation|GetActorLocation)))
  (LocalVariables|SetSquareBelow _square)
  (if (== _square 0)
    (return false false)
    (else
      (bind (_legal_move _piecetocapture) (Default|CanMakeMove (Variables|Default|GetBoard) self (Variables|/Game/Blueprints/BoardSquare.BoardSquare_C|GetX (LocalVariables|GetSquareBelow)) (Variables|/Game/Blueprints/BoardSquare.BoardSquare_C|GetY (LocalVariables|GetSquareBelow))))
      (if _legal_move
        (bind _output_get (Variables|Default|SetX (Variables|/Game/Blueprints/BoardSquare.BoardSquare_C|GetX (LocalVariables|GetSquareBelow))))
        (bind _output_get_2 (Variables|Default|SetY (Variables|/Game/Blueprints/BoardSquare.BoardSquare_C|GetY (LocalVariables|GetSquareBelow))))
        (bind _morejumps (Default|MakeMove (Variables|Default|GetBoard) self _output_get _output_get_2 _piecetocapture))
        (bind _center (Class|GameBoard|GetCenterOfIndex(Message) (Variables|Default|GetBoard) _output_get _output_get_2))
        (Variables|Default|SetTargetLocation _center)
        (return true _morejumps)
        (else
          (bind _center_2 (Class|GameBoard|GetCenterOfIndex(Message) (Variables|Default|GetBoard) (Variables|Default|GetX) (Variables|Default|GetY)))
          (Variables|Default|SetTargetLocation _center_2)
          (Development|PrintString (Utilities|String|Append "Illegal Move to: " "{" (Utilities|String|ToString(Integer) (Variables|/Game/Blueprints/BoardSquare.BoardSquare_C|GetX (LocalVariables|GetSquareBelow))) "," (Utilities|String|ToString(Integer) (Variables|/Game/Blueprints/BoardSquare.BoardSquare_C|GetY (LocalVariables|GetSquareBelow))) "}"))
          (return false false))))))

(fn SetSquareOver
  (params (Square :type Board%20Square%20Object%20Reference) (ValidMoveTarget :type Boolean))
  (if (not (== Square (Variables|Default|GetSquareOver)))
    (Default|SetHighlightState Square true ValidMoveTarget)
    (if (== (Variables|Default|GetSquareOver) 0)
      _
      (else
        (Default|SetHighlightState (Variables|Default|GetSquareOver) false false)))
    (Variables|Default|SetSquareOver Square)))

(fn ClearSquareOver
  (if (not (== 0 (Variables|Default|GetSquareOver)))
    (Default|SetHighlightState (Variables|Default|GetSquareOver) false false)
    (Variables|Default|SetSquareOver 0)))

(fn Despawn
  (Variables|Default|SetbAutoDestroyWhenFinished true)
  (return true))

(fn GetIndex
  (return (Variables|Default|GetX) (Variables|Default|GetY)))

(fn IsBlack
  (return (Variables|Default|GetBlack)))

(fn IsKing
  (return (Variables|Default|GetKing)))